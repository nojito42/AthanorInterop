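; Hexagon tile actor that highlights under the mouse cursor and carries a number label set through SetNumber.
; BeginPlay enables mouse-over events on the first player controller, and Mesh2 receives the cursor events.
; Hovering swaps Mesh1 for Mesh3 and enlarges the actor, widening X and Y relatively while forcing a fixed Z scale.
; Cursor exit reverses the swap and restores the transform cached by the construction script.
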(event OnBeginCursorOver(Mesh2)
  (params (TouchedComponent :type Primitive%20Component%20Object%20Reference))
  (bind _self self)
  (bind _returnvalue (Transformation|GetActorTransform _self))
  (bind _returnvalue_2 (* (.scale _returnvalue) "1.200000,1.200000,1.200000"))
  (Development|SetHiddeninGame (Variables|Default|GetMesh3) false false)
  (Development|SetHiddeninGame (Variables|Actor|GetMesh1) true false)
  (Transformation|SetActorTransform (Math|Transform|MakeTransform (.location _returnvalue) (.rotation _returnvalue) (Math|Vector|MakeVector (.x _returnvalue_2) (.y _returnvalue_2) 12.0))))

(event OnEndCursorOver(Mesh2)
  (params (TouchedComponent :type Primitive%20Component%20Object%20Reference))
  (Development|SetHiddeninGame (Variables|Default|GetMesh3) true false)
  (Development|SetHiddeninGame (Variables|Actor|GetMesh1) false false)
  (Transformation|SetActorTransform (Variables|Default|GetSpawnTransform)))

(event EventBeginPlay
  (Variables|/Script/Engine.PlayerController|SetbEnableMouseOverEvents (Game|GetPlayerController 0) true))

(event Collision|EventActorBeginOverlap
  (params (OtherActor :type Actor%20Object%20Reference)))

(event EventTick
  (params (DeltaSeconds :type Float%20%28single-precision%29)))

(fn ConstructionScript
  (Variables|Default|SetSpawnTransform (Transformation|GetActorTransform self)))

(fn SetNumber
  (params (NewParam :type Integer))
  (Rendering|Components|TextRender|SetText (Variables|Default|GetText) (Utilities|Text|ToText(Integer) NewParam)))