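; BP_AthanLogo is a logo actor that spins continuously in its own local space.
; Tick caches DeltaSeconds in a variable and passes the X, Y and Z variables as roll, pitch and yaw rates to the Rotate function.
; Rotate checks the DoRotate flag, then adds a local rotation scaled by the cached delta, keeping the spin frame-rate independent.
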(event EventBeginPlay)

(event Collision|EventActorBeginOverlap
  (params (OtherActor :type Actor%20Object%20Reference)))

(event EventTick
  (params (DeltaSeconds :type Float%20%28single-precision%29))
  (Variables|Default|SetDelta%20Seconds DeltaSeconds)
  (CallFunction|Rotate (Math|Rotator|MakeRotator (Variables|Default|GetX) (Variables|Default|GetY) (Variables|Default|GetZ))))

(fn ConstructionScript)

(fn Rotate
  (params (Rotator :type Rotator))
  (bind _delta_seconds (Variables|Default|GetDelta%20Seconds))
  (if (Variables|Default|GetDoRotate)
    (Transformation|AddActorLocalRotation (Math|Rotator|MakeRotator (* (.roll Rotator) _delta_seconds) (* (.pitch Rotator) _delta_seconds) (* (.yaw Rotator) _delta_seconds)) false false)))